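; BP_Measurement is a workbench tool actor that displays the distance between two points, PointA and PointB.
; Its Construction Script moves the first two spline points to those world positions and places the text label at their scaled sum, stored as MidPoint.
; The label shows the distance in centimeters, meters or feet according to DisplayUnit.
; The event graph holds only disabled stubs, so it adds no runtime logic.
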(fn `UserConstructionScript`
  (`SplineComponent.SetLocationAtSplinePoint` (`self.MeasurementSpline`) 0 (`self.PointA`) "World" true)
  (`SplineComponent.SetLocationAtSplinePoint` (`self.MeasurementSpline`) 1 (`self.PointB`) "World" true)
  (bind _output_get (set `self.MidPoint` (* (+ (`self.PointA`) (`self.PointB`)) (`self.NewVar`))))
  (`SceneComponent.K2_SetWorldLocation` (`self.DistanceText`) _output_get false false)
  (switch `/Workbench/Workbench/Tools/WORKBENCH_By_Venkatesh_Lokhande/Enumerations/E_MeasurementUnit` (`self.DisplayUnit`)
    (:`NewEnumerator0`
      (`TextRenderComponent.K2_SetText` (`self.DistanceText`) (`|FormatText` "Distance : {Distance}cm" (`KismetTextLibrary.Conv_DoubleToText` (`KismetMathLibrary.Vector_Distance` (`self.PointA`) (`self.PointB`)) "HalfToEven"))))
    (:`NewEnumerator1`
      (`TextRenderComponent.K2_SetText` (`self.DistanceText`) (`|FormatText` "Distance : {Distance}m" (`KismetTextLibrary.Conv_DoubleToText` (/ (`KismetMathLibrary.Vector_Distance` (`self.PointA`) (`self.PointB`)) 100.0) "HalfToEven"))))
    (:`NewEnumerator2`
      (`TextRenderComponent.K2_SetText` (`self.DistanceText`) (`|FormatText` "Distance : {Distance}ft" (`KismetTextLibrary.Conv_DoubleToText` (/ (`KismetMathLibrary.Vector_Distance` (`self.PointA`) (`self.PointB`)) 30.48) "HalfToEven"))))))